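; BP_FlockTarget is an actor that wanders an A* node network, presumably as the target a flock follows.
; Two seconds after BeginPlay, Tick starts sending its AStar to a random node, after a short delay, whenever it is not moving.
; The validity check, path request and debug print each roll their own random index, so their nodes can differ.
; A FlipFlop toggles node visibility, but its P-key trigger is disconnected.
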(event Custom|ToggleVisibility
  (bind _astar (Variables|Default|GetAStar))
  (bind _astarglobals (Variables|/Script/CoastSim.AStarComponent|GetAStarGlobals _astar))
  (bind _astarnodes (Variables|/Script/CoastSim.AStarGlobals|GetAStarNodes _astarglobals))
  (Utilities|FlowControl|FlipFlop
    (:A
      (for _array_element _astarnodes
        (Rendering|SetActorHiddenInGame _array_element false)))
    (:B
      (for _array_element_2 _astarnodes
        (Rendering|SetActorHiddenInGame _array_element_2 true)))))

(event Custom|Tick2
  ;[0.15 0.15 0.15 0.5] Hide or Show AStar Nodes
)

(event EventBeginPlay
  (Utilities|FlowControl|Delay 2.0)
  (Variables|Default|Sethasstarted true))

(event Collision|EventActorBeginOverlap
  (params (OtherActor :type Actor%20Object%20Reference)))

(event EventTick
  (params (DeltaSeconds :type Float%20%28single-precision%29))
  (bind _astar (Variables|Default|GetAStar))
  (bind _astarglobals (Variables|/Script/CoastSim.AStarComponent|GetAStarGlobals _astar))
  (bind _astarnodes (Variables|/Script/CoastSim.AStarGlobals|GetAStarNodes _astarglobals))
  (bind _returnvalue (Utilities|Array|Length _astarnodes))
  (bind _returnvalue_2 (Math|Random|RandomInteger _returnvalue))
  (bind _output (Utilities|Array|Get(acopy) _astarnodes _returnvalue_2))
  (CallFunction|Tick2)
  (if (Variables|Default|Gethasstarted)
    (if (not (Variables|/Script/CoastSim.AStarComponent|GetbIsMoving (Variables|Default|GetAStar)))
      ;[0.15 0.15 0.15 0.5] Gets random node to go to
      (Utilities|FlowControl|Delay 0.2)
      (if (Utilities|IsValid _output)
        (Class|AStarComponent|PathFindto (Variables|Default|GetAStar) _output)
        (Development|PrintString (Utilities|GetDisplayName _output))))))

(fn ConstructionScript)