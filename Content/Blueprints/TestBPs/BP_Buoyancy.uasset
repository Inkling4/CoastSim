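; Test Blueprint actor that configures a NewBuoyancy component to act on its static mesh.
; The Construction Script passes the mesh to the component, then uses nested loops to append a flat, evenly spaced grid of pontoon locations, centered on Y and extending along positive X.
; An older hardcoded four-point layout is left disconnected, and the Event Graph has no active logic.
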(event EventBeginPlay)

(event Collision|EventActorBeginOverlap
  (params (OtherActor :type Actor%20Object%20Reference)))

(event EventTick
  (params (DeltaSeconds :type Float%20%28single-precision%29)))

(fn ConstructionScript
  (Variables|/Script/CoastSim.NewBuoyancyComponent|SetMyStaticMeshComponent (Variables|Default|GetNewBuoyancy) (Variables|Default|GetStaticMesh))
  (for _index (range 0 4)
    (for _index_2 (range 0 2)
      (Utilities|Array|Add (Variables|/Script/CoastSim.NewBuoyancyComponent|GetPontoonsLocations (Variables|Default|GetNewBuoyancy)) (Math|Vector|MakeVector (Math|Conversions|ToFloat(Integer) (* _index 3e+02)) (Math|Conversions|ToFloat(Integer) (- (* _index_2 3e+02) 3e+02)) 0.0)))))