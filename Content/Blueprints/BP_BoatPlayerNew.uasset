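; Player-controlled rowboat pawn that moves on a physics Box, with a Buoyancy component fed the boat's static mesh.
; Enhanced Input (IMC_Rowman) drives look, forward/backward acceleration forces and direct yaw rotation, with rowing and turning ramped over the first second held.
; On release, a timeline replays the last yaw step to ease out turns.
; Tick projects velocity onto the Box's forward vector, removing sideways drift so momentum follows the heading.
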(event Input|EnhancedActionEvents|EnhancedInputActionIA_Move
  (params (ActionValue :type Float%20%28double-precision%29) (ElapsedSeconds :type Float%20%28double-precision%29) (TriggeredSeconds :type Float%20%28double-precision%29) (InputAction :type Input%20Action%20Object%20Reference :default "/Game/Input/IA_Move.IA_Move"))
  (bind _staticmesh (Variables|Default|GetStaticMesh))
  (bind _box (Variables|Default|GetBox))
  (bind _backwardrowforece (Variables|Default|GetBackwardRowForece))
  (bind _forwardrowforce (Variables|Default|GetForwardRowForce))
  (bind _staticmesh_2 (Variables|Default|GetStaticMesh))
  (bind _returnvalue (|SmoothMove_2 ActionValue TriggeredSeconds _backwardrowforece))
  (bind _returnvalue_2 (|SmoothMove_2_3 ActionValue TriggeredSeconds _forwardrowforce))
  (bind (_returnvalue_x _returnvalue_y) (|CalculateForwardForce_3 _staticmesh _returnvalue_2))
  (bind (_returnvalue_x_2 _returnvalue_y_2) (|CalculateBackwardForce_3 _staticmesh_2 _returnvalue))
  ;[0.15 0.15 0.15 0.5] Forward/backward Movement using physics
  (if (> ActionValue 0.0)
    (Physics|AddForce _box (Math|Vector|MakeVector _returnvalue_x _returnvalue_y 0.0) "None" true)
    (else
      (Physics|AddForce _box (Math|Vector|MakeVector _returnvalue_x_2 _returnvalue_y_2 0.0) "None" true))))

(event Input|EnhancedActionEvents|EnhancedInputActionIA_Look
  (params (ActionValue :type Vector%202D%20Structure) (ElapsedSeconds :type Float%20%28double-precision%29) (TriggeredSeconds :type Float%20%28double-precision%29) (InputAction :type Input%20Action%20Object%20Reference :default "/Game/Input/IA_Look.IA_Look"))
  (bind _looksensitivity (Variables|Default|GetLooksensitivity))
  ;[0.15 0.15 0.15 0.5] Look
  (Pawn|Input|AddControllerPitchInput (* (* (.x ActionValue) _looksensitivity) -1.0))
  (Pawn|Input|AddControllerYawInput (* (.y ActionValue) _looksensitivity)))

(event Input|EnhancedActionEvents|EnhancedInputActionIA_Rotate
  (params (ActionValue :type Float%20%28double-precision%29) (ElapsedSeconds :type Float%20%28double-precision%29) (TriggeredSeconds :type Float%20%28double-precision%29) (InputAction :type Input%20Action%20Object%20Reference :default "/Game/Input/IA_Rotate.IA_Rotate"))
  (bind _returnvalue (Math|Float|Clamp(Float) TriggeredSeconds))
  (bind _rotationstrength (Variables|Default|GetRotationStrength))
  (bind _returnvalue_2 (* ActionValue _rotationstrength))
  (bind _returnvalue_3 (Math|Float|Lerp 0.0 _returnvalue_2 _returnvalue))
  ;[0.15 0.15 0.15 0.5] Rotation
  (:Triggered
    (Class|Actor|AddActorWorldRotation (Math|Rotator|MakeRotator 0.0 0.0 _returnvalue_3))
    (Variables|Default|SetLastDeltaRotation _returnvalue_3))
  (:Started
    (bind _newtrack_0 (Timeline|Timeline Stop)
      (:Update
        (Class|Actor|AddActorWorldRotation (Math|Rotator|MakeRotator 0.0 0.0 (Math|Float|Lerp 0.0 (Variables|Default|GetLastDeltaRotation) _newtrack_0))))))
  (:Completed
    (Timeline|Timeline PlayFromStart)))

(event EventBeginPlay
  ;[0.15 0.15 0.15 0.5] Bind InputMapping
  (bind _asplayer_controller (Utilities|Casting|CastToPlayerController (Pawn|GetController)))
  (Utilities|IsValid (PlayerController|LocalPlayerSubsystems|GetEnhancedInputLocalPlayerSubsystem _asplayer_controller)
    (:Is%20Valid
      (Input|AddMappingContext (PlayerController|LocalPlayerSubsystems|GetEnhancedInputLocalPlayerSubsystem _asplayer_controller) "/Game/Input/IMC_Rowman.IMC_Rowman" 0 "(bIgnoreAllPressedKeysUntilRelease=True,bForceImmediately=False,bNotifyUserSettings=False)"))))

(event EventTick
  (params (DeltaSeconds :type Float%20%28single-precision%29))
  (bind _box (Variables|Default|GetBox))
  (bind _returnvalue (Math|Vector|GetForwardVector _box))
  ;[0.15 0.15 0.15 0.5] Align physics to current view direction
  (bind _returnvalue_2 (Physics|GetPhysicsLinearVelocity _box "None"))
  (Physics|SetPhysicsLinearVelocity _box (* (Math|Vector|DotProduct _returnvalue_2 _returnvalue) _returnvalue) false "None"))

(fn ConstructionScript
  (Variables|/Script/CoastSim.NewBuoyancyComponent|SetMyStaticMeshComponent (Variables|Default|GetBuoyancy) (Variables|Default|GetStaticMesh)))