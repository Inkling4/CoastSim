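; AI boat that wanders the map on its own, pathfinding to random A* nodes.
; After a short startup delay, Tick sends the AStar component to a random global node whenever it is idle, re-rolling the random index at each use.
; Tick also slowly interpolates the actor's yaw toward the movement direction and periodically samples its location.
; The construction script hands the Boat mesh to the Buoyancy component.
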(event EventBeginPlay
  (Utilities|FlowControl|Delay 2.0)
  (Variables|Default|Sethasstarted true))

(event Collision|EventActorBeginOverlap
  (params (OtherActor :type Actor%20Object%20Reference)))

(event EventTick
  (params (DeltaSeconds :type Float%20%28single-precision%29))
  (bind _returnvalue (Math|Random|RandomInteger 255))
  (bind _astar (Variables|Default|GetAStar))
  (bind _astar_2 (Variables|Default|GetAStar))
  (bind _boat (Variables|Default|GetBoat))
  (bind _returnvalue_2 (Transformation|GetWorldLocation _boat))
  (bind _astarglobals (Variables|/Script/CoastSim.AStarComponent|GetAStarGlobals _astar))
  (bind _movementdirection (Variables|/Script/CoastSim.AStarComponent|GetMovementDirection _astar_2))
  (bind _astarnodes (Variables|/Script/CoastSim.AStarGlobals|GetAStarNodes _astarglobals))
  (bind _output (Utilities|Array|Get(acopy) _astarnodes _returnvalue))
  (Utilities|FlowControl|Sequence
    (:then_0
      (if (Variables|Default|Gethasstarted)
        (if (not (Variables|/Script/CoastSim.AStarComponent|GetbIsMoving (Variables|Default|GetAStar)))
          (Utilities|FlowControl|Delay 0.2)
          (if (Utilities|IsValid _output)
            (Class|AStarComponent|PathFindto (Variables|Default|GetAStar) _output)
            (Development|PrintString (Utilities|GetDisplayName _output))))))
    (:then_1
      (Utilities|FlowControl|DoOnce false :!label _label
        (:Completed
          (bind _output_get (Variables|Default|SetNewLoc (Transformation|GetActorLocation)))
          (Utilities|FlowControl|Delay 0.2)
          (Variables|Default|SetOldLoc _output_get)
          (goto _label Reset))))
    (:then_2
      (Transformation|SetActorRotation (Math|Interpolation|RInterpTo (Math|Rotator|MakeRotator 0.0 0.0 (.yaw (Transformation|GetWorldRotation _boat))) (Math|Rotator|MakeRotator 0.0 0.0 (.yaw (Math|Rotator|FindLookatRotation _returnvalue_2 (+ _returnvalue_2 (Math|Vector|MakeVector (.x _movementdirection) (.y _movementdirection) 0.0))))) DeltaSeconds 0.2)))))

(fn ConstructionScript
  (Variables|/Script/CoastSim.NewBuoyancyComponent|SetMyStaticMeshComponent (Variables|Default|GetBuoyancy) (Variables|Default|GetBoat)))