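; BP_PlayerBoat is the player-controlled boat, driven through Enhanced Input with the IMC_Rowman mapping context added on BeginPlay.
; IA_Move sets the transform directly: X shifts it along its facing without sweep, and Y adds yaw while zeroing pitch and roll.
; Steps scale by Speed and RotationSpeed but not delta time, and turning prints a debug string.
; The construction script hands the static mesh to the Buoyancy component.
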(event Input|EnhancedActionEvents|EnhancedInputActionIA_Move
  (params (ActionValue :type Vector%202D%20Structure) (ElapsedSeconds :type Float%20%28double-precision%29) (TriggeredSeconds :type Float%20%28double-precision%29) (InputAction :type Input%20Action%20Object%20Reference :default "/Game/Input/IA_Move.IA_Move"))
  (bind _returnvalue (Transformation|GetActorRotation))
  (bind _speed (Variables|Default|GetSpeed))
  (bind _returnvalue_2 (* ActionValue _speed))
  (bind (_x _y) (Math|Vector2D|BreakVector2D _returnvalue_2))
  (if (!= _x 0.0)
    (Transformation|SetActorLocation (+ (Math|Vector|RotateVector (Math|Vector|MakeVector _x 0.0 0.0) _returnvalue) (Transformation|GetActorLocation)) false false))
  (if (!= _y 0.0)
    (Transformation|SetActorRotation (Math|Rotator|MakeRotator 0.0 0.0 (+ (* _y (Variables|Default|GetRotationSpeed)) (.Yaw (Math|Rotator|BreakRotator _returnvalue)))))
    (Development|PrintString "Rotating")))

(event EventBeginPlay
  (bind _asplayer_controller (Utilities|Casting|CastToPlayerController (Pawn|GetController)))
  (Utilities|IsValid (PlayerController|LocalPlayerSubsystems|GetEnhancedInputLocalPlayerSubsystem _asplayer_controller)
    (:Is%20Valid
      (Input|AddMappingContext (PlayerController|LocalPlayerSubsystems|GetEnhancedInputLocalPlayerSubsystem _asplayer_controller) "/Game/Input/IMC_Rowman.IMC_Rowman" 0 "(bIgnoreAllPressedKeysUntilRelease=True,bForceImmediately=False,bNotifyUserSettings=False)"))))

(event Collision|EventActorBeginOverlap
  (params (OtherActor :type Actor%20Object%20Reference)))

(event EventTick
  (params (DeltaSeconds :type Float%20%28single-precision%29)))

(fn ConstructionScript
  (Variables|/Script/CoastSim.NewBuoyancyComponent|SetMyStaticMeshComponent (Variables|Default|GetBuoyancy) (Variables|Default|GetStaticMesh)))