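; BP_NodeSpawner fills the area of its Box component with a flat grid of BP_AStarNode actors.
; UpdateSpawnNumbers derives row and column counts and spawn scale from the box extent and NodeSize.
; SpawnNodes uses nested loops to place scaled nodes from the box's minimum X/Y corner at its center height, storing them in OwnedNodes.
; DeleteOwnedNodes prints and destroys each stored node, without clearing the array.
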(event Custom|SpawnNodes
  (bind _box (Variables|Default|GetBox))
  (bind _returnvalue (Components|Box|GetScaledBoxExtent _box))
  (bind _returnvalue_2 (Transformation|GetWorldLocation _box))
  (for _index (range 0 (Variables|Default|GetNumberOfNodeColumn))
    (for _index_2 (range 0 (Variables|Default|GetNumberOfNodeRow))
      (bind _returnvalue_3 (Game|SpawnActorfromClass "/Game/Blueprints/BP_AStarNode.BP_AStarNode_C" (Math|Transform|MakeTransform (Math|Vector|MakeVector (+ (* _index_2 (* (Variables|Default|GetNodeSize) 50)) (- (.x _returnvalue_2) (.x _returnvalue))) (+ (* _index (* (Variables|Default|GetNodeSize) 50)) (- (.y _returnvalue_2) (.y _returnvalue))) (.z _returnvalue_2)) "0, 0, 0" (Variables|Default|GetSpawn%20Size)) "Undefined" "MultiplyWithRoot" self 0))
      (Utilities|Array|Add (Variables|Default|GetOwnedNodes) _returnvalue_3))))

(event Custom|UpdateSpawnNumbers
  (bind _box (Variables|Default|GetBox))
  (bind _returnvalue (Components|Box|GetScaledBoxExtent _box))
  (Variables|Default|SetNumberOfNodeRow (Math|Float|Floor (/ (.x _returnvalue) (* (Variables|Default|GetNodeSize) 25))))
  (Variables|Default|SetNumberOfNodeColumn (Math|Float|Floor (/ (.y _returnvalue) (* (Variables|Default|GetNodeSize) 25))))
  (Variables|Default|SetSpawn%20Size (* "1.000000,1.000000,1.000000" (Variables|Default|GetNodeSize))))

(event Custom|DeleteOwnedNodes
  (for _array_element (Variables|Default|GetOwnedNodes)
    (Development|PrintString (Utilities|GetDisplayName _array_element))
    (Actor|DestroyActor _array_element)))

(event Collision|EventActorBeginOverlap
  (params (OtherActor :type Actor%20Object%20Reference)))

(event EventTick
  (params (DeltaSeconds :type Float%20%28single-precision%29)))

(fn ConstructionScript)